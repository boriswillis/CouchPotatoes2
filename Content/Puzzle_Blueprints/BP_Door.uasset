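; BP_Door is a puzzle door that slides open and closed on Interact, but only after PickUpKey has set HasKey.
; A FlipFlop alternately plays and reverses DoorTimeline.
; The timeline's DoorSlide track drives the actor's relative X, with Y and Z taken from the StaticMesh's relative location.
; An unconnected mesh rotation node is left unused.
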(event EventInteract
  (bind _staticmesh (Variables|Default|GetStaticMesh))
  (bind _relativelocation (Variables|/Script/Engine.SceneComponent|GetRelativeLocation _staticmesh))
  (if (Variables|Default|GetHasKey?)
    (Utilities|FlowControl|FlipFlop
      (:A
        (bind _door_slide (Timeline|Door%20Timeline Play)
          (:Update
            (Transformation|SetActorRelativeLocation (Math|Vector|MakeVector _door_slide (.y _relativelocation) (.z _relativelocation))))))
      (:B
        (Timeline|Door%20Timeline Reverse)))))

(event EventPickUpKey
  (Variables|Default|SetHasKey? true))

(fn ConstructionScript)